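; BP_EnemyGOD is an enemy spawner that creates BP_Enemy actors at its own location at random intervals.
; Tick accumulates elapsed time and, once it exceeds CreateTime, resets the timer and spawns an enemy.
; SetCreateTime picks the next interval between MinTime and MaxTime, both on BeginPlay and after each spawn.
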(event `self.ReceiveBeginPlay`
  (`self.SetCreateTime`))

(event `self.ReceiveTick`
  (params (DeltaSeconds :type "Float (single-precision)"))
  ; 시간이 흐른다.
  (set `self.CurrentTime` (+ DeltaSeconds (`self.CurrentTime`)))
  ; 생성시간을 초과했다면
  (if (> (`self.CurrentTime`) (`self.CreateTime`))
    ; 경과시간 초기화
    (set `self.CurrentTime` 0.0)
    ; 적을 만들고 싶다.
    (`|SpawnActorFromClass` "/Game/Blueprints/BP_Enemy.BP_Enemy_C" (`KismetMathLibrary.MakeTransform` (`self.K2_GetActorLocation`)) "Undefined" "MultiplyWithRoot" null null)
    ; 생성시간 재설정
    (`self.SetCreateTime`)))

(fn `SetCreateTime`
  (set `self.CreateTime` (`KismetMathLibrary.RandomFloatInRange` (`self.MinTime`) (`self.MaxTime`))))

(fn `UserConstructionScript`)